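; BP_DoorMain is a door actor in the residential house that the player opens and closes with either motion controller trigger.
; Overlapping its trigger volume enables input and opens a Gate, while leaving disables input without closing that Gate.
; Each gated press runs a FlipFlop that toggles PlayerNear on the door mesh's AnimBPDoorMain animation Blueprint, which presumably drives the door motion.
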(event OnComponentBeginOverlap(Trigger)
  (params (OverlappedComponent :type Primitive%20Component%20Object%20Reference) (OtherActor :type Actor%20Object%20Reference) (OtherComp :type Primitive%20Component%20Object%20Reference) (OtherBodyIndex :type Integer) (bFromSweep :type Boolean) (SweepResult :type Hit%20Result%20Structure%20%28by%20ref%29))
  (Input|EnableInput (Game|GetPlayerController 0))
  (Utilities|FlowControl|Gate true) ; enters at Open
)

(event OnComponentEndOverlap(Trigger)
  (params (OverlappedComponent :type Primitive%20Component%20Object%20Reference) (OtherActor :type Actor%20Object%20Reference) (OtherComp :type Primitive%20Component%20Object%20Reference) (OtherBodyIndex :type Integer))
  (Input|DisableInput (Game|GetPlayerController 0)))

(event Input|KeyboardEvents|MotionControllerLeftTrigger
  (params (Key :type Key%20Structure))
  (:Pressed
    (Utilities|FlowControl|Gate true
      (:Exit
        (bind _asanim_bpdoor_main (Utilities|Casting|CastToAnimBPDoorMain (Components|SkeletalMesh|GetAnimInstance (Variables|Default|GetDoor_main))))
        (Utilities|FlowControl|FlipFlop
          (:A
            (Variables|/Game/HQ_ResidentialHouse/Meshes/DoorMain/AnimBPDoorMain.AnimBPDoorMain_C|SetPlayerNear _asanim_bpdoor_main true))
          (:B
            (Variables|/Game/HQ_ResidentialHouse/Meshes/DoorMain/AnimBPDoorMain.AnimBPDoorMain_C|SetPlayerNear _asanim_bpdoor_main false)))))))

(event Input|KeyboardEvents|MotionControllerRightTrigger
  (params (Key :type Key%20Structure))
  (:Pressed
    (Utilities|FlowControl|Gate true
      (:Exit
        (bind _asanim_bpdoor_main (Utilities|Casting|CastToAnimBPDoorMain (Components|SkeletalMesh|GetAnimInstance (Variables|Default|GetDoor_main))))
        (Utilities|FlowControl|FlipFlop
          (:A
            (Variables|/Game/HQ_ResidentialHouse/Meshes/DoorMain/AnimBPDoorMain.AnimBPDoorMain_C|SetPlayerNear _asanim_bpdoor_main true))
          (:B
            (Variables|/Game/HQ_ResidentialHouse/Meshes/DoorMain/AnimBPDoorMain.AnimBPDoorMain_C|SetPlayerNear _asanim_bpdoor_main false)))))))

(fn ConstructionScript)