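; Point-and-click VR keyboard Blueprint that hosts the WBP_PointAndClick widget in its WidgetKeyboard component.
; On BeginPlay it casts that widget, gives it the Widget Interaction component and binds handlers for the Browser, Enter, ChatBox and Change Theme buttons.
; A failed cast prints an error.
; The four handler events are empty here, so browser and chat box toggling, message sending and theming are not implemented in this graph.
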(event Custom|ToggleBrowserVisability
  ;[1 1 1] // Bind Events for when the 'Enter,' 'Browser' and 'Change Theme' buttons are pressed
)

(event Custom|ToggleChatBoxVisability
  ;[1 1 1] // Bind Events for when the 'Enter,' 'Browser' and 'Change Theme' buttons are pressed
)

(event Custom|ChangeTheme
  (params (ThemeToUse :type Struct%20Blank%20Button%20Styles%20Structure))
  ;[1 1 1] // Bind Events for when the 'Enter,' 'Browser' and 'Change Theme' buttons are pressed
  ;;[1 1 1] // Call Change Theme interface on BP_ChatBox
)

(event Custom|SendMessageToChatBox
  (params (MessageToSend :type Text))
  ;[1 1 1] // Bind Events for when the 'Enter,' 'Browser' and 'Change Theme' buttons are pressed
)

(event EventBeginPlay
  ;[1 1 1] // Give the Keyboard widget a reference to the Widget Interaction Component.
  (bind _aswbp_point_and_click (Utilities|Casting|CastToWBP_PointAndClick (UserInterface|GetUserWidgetObject (Variables|Default|GetWidget_Keyboard)))
    (:then
      (Variables|/Game/VRKeyboard/Keyboards/PointAndClick/Blueprints/Keyboard/Widgets/WBP_PointAndClick.WBP_PointAndClick_C|SetWidgetInteraction _aswbp_point_and_click (Variables|Default|GetWidgetInteractionComponent))
      ;[1 1 1] // Bind Events for when the 'Enter,' 'Browser' and 'Change Theme' buttons are pressed
      (EventDispatchers|BindEventtoBrowserButtonPressed _aswbp_point_and_click (delegate Custom|ToggleBrowserVisability))
      (EventDispatchers|BindEventtoEnterButtonPressed _aswbp_point_and_click (delegate Custom|SendMessageToChatBox))
      (EventDispatchers|BindEventtoChatBoxButtonPressed _aswbp_point_and_click (delegate Custom|ToggleChatBoxVisability))
      ;;[1 1 1] // Call Change Theme interface on BP_ChatBox
      (EventDispatchers|BindEventtoChangeThemeButtonPressed _aswbp_point_and_click (delegate Custom|ChangeTheme)))
    (:CastFailed
      ;[1 1 0] // If the cast failed it's because the Widget_Keyboard component didn't have the Widget Class option set to the correct widget.
      (Development|PrintString "BP_VRKeyboard//Cast Failed"))))

(fn ConstructionScript)