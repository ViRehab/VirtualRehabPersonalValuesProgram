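; BP_StartScavenger is the start trigger for a scavenger hunt game.
; The first overlap with its static mesh, gated by a DoOnce, plays SCChest and toggles visibility on the start and directions meshes, planes and widgets.
; It then finds every BP_TreasureChest_Start actor and sets GameActive to true, switching the treasure chests into play.
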(event OnComponentBeginOverlap(StaticMesh)
  (params (OverlappedComponent :type Primitive%20Component%20Object%20Reference) (OtherActor :type Actor%20Object%20Reference) (OtherComp :type Primitive%20Component%20Object%20Reference) (OtherBodyIndex :type Integer) (bFromSweep :type Boolean) (SweepResult :type Hit%20Result%20Structure%20%28by%20ref%29))
  (Utilities|FlowControl|DoOnce false
    (:Completed
      (Audio|Components|Audio|Play (Variables|Default|GetSC_Chest) 0.0)
      (Rendering|ToggleVisibility (Variables|Default|GetStaticMesh) false)
      (bind _outactors (Actor|GetAllActorsOfClass "/Game/ARS/Blueprints/BP_TreasureChest_Start.BP_TreasureChest_Start_C"))
      (for _array_element _outactors
        (Variables|/Game/ARS/Blueprints/BP_TreasureChest_Start.BP_TreasureChest_Start_C|SetGameActive _array_element true)))))

(event EventBeginPlay)

(fn ConstructionScript)