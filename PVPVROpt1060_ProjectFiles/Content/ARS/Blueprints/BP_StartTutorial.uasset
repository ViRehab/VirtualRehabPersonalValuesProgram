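; Tutorial trigger actor that plays one-shot audio cues and reveals a treasure chest as the player progresses.
; Box overlap plays the coin cue and toggles visibility of the key tutorial and box.
; StaticMesh overlap, gated on the first BP_PickupRC being grabbed, plays the chest cue, swaps in the chest mesh and toggles the same components.
; It then chains delayed CB and Transport cues before setting CanTransport.
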(event OnComponentBeginOverlap(Box)
  (params (OverlappedComponent :type Primitive%20Component%20Object%20Reference) (OtherActor :type Actor%20Object%20Reference) (OtherComp :type Primitive%20Component%20Object%20Reference) (OtherBodyIndex :type Integer) (bFromSweep :type Boolean) (SweepResult :type Hit%20Result%20Structure%20%28by%20ref%29))
  (Utilities|FlowControl|DoOnce false
    (:Completed
      (Audio|Components|Audio|Play (Variables|Default|GetSC_Coin) 0.0)
      (Rendering|ToggleVisibility (Variables|Default|GetKeyTutorial) false))))

(event OnComponentBeginOverlap(StaticMesh)
  (params (OverlappedComponent :type Primitive%20Component%20Object%20Reference) (OtherActor :type Actor%20Object%20Reference) (OtherComp :type Primitive%20Component%20Object%20Reference) (OtherBodyIndex :type Integer) (bFromSweep :type Boolean) (SweepResult :type Hit%20Result%20Structure%20%28by%20ref%29))
  (bind _outactors (Actor|GetAllActorsOfClass "/Game/VirtualRealityBP/Blueprints/BP_PickupRC.BP_PickupRC_C"))
  (if (Variables|/Game/VirtualRealityBP/Blueprints/BP_PickupRC.BP_PickupRC_C|GetRCGrabbed (Utilities|Array|Get(acopy) _outactors))
    (Utilities|FlowControl|DoOnce false
      (:Completed
        (Audio|Components|Audio|Play (Variables|Default|GetSC_Chest) 0.0)
        (Components|StaticMesh|SetStaticMesh (Variables|Default|GetTutorialChest) "/Game/ARS/Geometry/SM_TreasureChest.SM_TreasureChest")
        (Rendering|ToggleVisibility (Variables|Default|GetKeyTutorial) false)
        (Utilities|FlowControl|Delay 7.0)
        (Audio|Components|Audio|Play (Variables|Default|GetCB) 0.0)
        (Utilities|FlowControl|Delay 45.0)
        (Audio|Components|Audio|Play (Variables|Default|Gettransport) 0.0)
        (Utilities|FlowControl|Delay 5.0)
        (Variables|Default|SetCanTransport true)))))

(event EventBeginPlay)

(event Collision|EventActorBeginOverlap
  (params (OtherActor :type Actor%20Object%20Reference)))

(event EventTick
  (params (DeltaSeconds :type Float%20%28single-precision%29)))

(fn ConstructionScript)