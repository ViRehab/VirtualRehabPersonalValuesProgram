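; BP_TreasureChest_Start is a VR treasure chest pickup that appears once the game is active and awards points when opened.
; Tick polls GameActive, then sets the chest mesh once and toggles the text, collision and key visibility.
; The first active overlap plays a coin sound, toggles those components again and increments the MotionControllerPawn's score and chest count.
; It also hides the chest on the left controller's iPad map widget and records a Google analytics event.
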(event OnComponentBeginOverlap(Collision)
  (params (OverlappedComponent :type Primitive%20Component%20Object%20Reference) (OtherActor :type Actor%20Object%20Reference) (OtherComp :type Primitive%20Component%20Object%20Reference) (OtherBodyIndex :type Integer) (bFromSweep :type Boolean) (SweepResult :type Hit%20Result%20Structure%20%28by%20ref%29))
  (bind _returnvalue (Game|Player|GetPlayerPawn 0))
  (bind _asmotion_controller_pawn (Utilities|Casting|CastToMotionControllerPawn _returnvalue))
  (if (Variables|Default|GetGameActive)
    (Utilities|FlowControl|DoOnce false
      (:Completed
        (Audio|Components|Audio|Play (Variables|Default|GetSC_Coin) 0.0)
        (Rendering|ToggleVisibility (Variables|Default|GetTextRender) false)
        (Default|AwardPoints (.AsMotion%20Controller%20Pawn (Utilities|Casting|CastToMotionControllerPawn (Game|Player|GetPlayerPawn 0))) 10)
        (CallFunction|RemovefromMap)
        (bind _output_get (Variables|/Game/VirtualRealityBP/Blueprints/MotionControllerPawn.MotionControllerPawn_C|SetChestOpened _asmotion_controller_pawn (+ (Variables|/Game/VirtualRealityBP/Blueprints/MotionControllerPawn.MotionControllerPawn_C|GetChestOpened _asmotion_controller_pawn) 1)))
        (Class|GoogleAnalyticsBlueprintLibrary|RecordGoogleEvent "Interaction" "Open Chest" "" _output_get)))))

(event Custom|RemoveFromMap
  (bind _outactors (Actor|GetAllActorsOfClass "/Game/VirtualRealityBP/Blueprints/MotionControllerPawn.MotionControllerPawn_C"))
  (bind _aswidget_ipad (Utilities|Casting|CastToWidget_Ipad (UserInterface|GetUserWidgetObject (Variables|/Game/VirtualRealityBP/Blueprints/BP_MotionController.BP_MotionController_C|GetWidget (Variables|/Game/VirtualRealityBP/Blueprints/MotionControllerPawn.MotionControllerPawn_C|GetLeftController (Utilities|Array|Get(acopy) _outactors))))))
  (Default|HideChestinMap _aswidget_ipad (Variables|Default|GetName)))

(event EventTick
  (params (DeltaSeconds :type Float%20%28single-precision%29))
  (Utilities|FlowControl|Delay 0.2)
  (if (Variables|Default|GetGameActive)
    (Utilities|FlowControl|DoOnce false
      (:Completed
        (Components|StaticMesh|SetStaticMesh (Variables|Default|GetStaticMesh) "/Game/ARS/Geometry/SM_TreasureChest.SM_TreasureChest")
        (Rendering|ToggleVisibility (Variables|Default|GetTextRender) false)))))

(fn ConstructionScript)