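; Basket target for a basket minigame that registers a score when a BP_PickupStone enters its sphere trigger.
; The overlap calls Activate, which reveals the point light and text, plays a sound, and calls AddBasket on the first BP_BasketGame's widget, then sets Active.
; Active is never checked here, so repeat overlaps count again.
; Deactivate hides the light and text but leaves Active unchanged.
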(event OnComponentBeginOverlap(Sphere)
  (params (OverlappedComponent :type Primitive%20Component%20Object%20Reference) (OtherActor :type Actor%20Object%20Reference) (OtherComp :type Primitive%20Component%20Object%20Reference) (OtherBodyIndex :type Integer) (bFromSweep :type Boolean) (SweepResult :type Hit%20Result%20Structure%20%28by%20ref%29))
  (if (== (Utilities|GetClass OtherActor) "/Game/ARS/Blueprints/BP_PickupStone.BP_PickupStone_C")
    (CallFunction|Activate)
    (Variables|Default|Setactive true)))

(event Custom|Activate
  (Development|SetHiddeninGame (Variables|Default|GetPointLight) false false)
  (Audio|PlaySound2D "/Game/Sounds/SC_BasketSound.SC_BasketSound")
  (bind _outactors (Actor|GetAllActorsOfClass "/Game/ARS/Blueprints/BP_BasketGame.BP_BasketGame_C"))
  (Default|AddBasket (.AsWidget%20Basket%20Game (Utilities|Casting|CastToWidget_BasketGame (UserInterface|GetUserWidgetObject (Variables|/Game/ARS/Blueprints/BP_BasketGame.BP_BasketGame_C|GetWidget (Utilities|Array|Get(acopy) _outactors)))))))

(event Custom|Deactivate
  (Development|SetHiddeninGame (Variables|Default|GetPointLight) true false))

(fn ConstructionScript)