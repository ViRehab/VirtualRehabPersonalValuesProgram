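; BP_Quiz2 is a quiz display actor that toggles between a question mark and a holographic quiz panel.
; A looping timer spins the question mark continuously.
; ShowQuiz and HideQuiz, which nothing in this graph calls, swap the question mark for the mesh, hologram base and widget, and play or stop the Netflix component.
; Leftover unconnected nodes would yaw a plane relative to the motion-controller pawn's camera.
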(event Custom|QM%20Rotator
  (Transformation|AddLocalRotation (Variables|Default|GetQuestionMark) "0,1.000000, 0" false false))

(event Custom|ShowQuiz
  (Development|SetHiddeninGame (Variables|Default|GetQuestionMark) true false)
  (Development|SetHiddeninGame (Variables|Default|GetStaticMesh) false false)
  (Development|SetHiddeninGame (Variables|Default|GetWidget) false false)
  (Audio|Components|Audio|Play (Variables|Default|GetNetflix) 0.0))

(event Custom|HideQuiz
  (Development|SetHiddeninGame (Variables|Default|GetQuestionMark) false false)
  (Development|SetHiddeninGame (Variables|Default|GetStaticMesh) true false)
  (Development|SetHiddeninGame (Variables|Default|GetWidget) true false)
  (Audio|Components|Audio|Stop (Variables|Default|GetNetflix)))

(event EventBeginPlay
  (Utilities|Time|SetTimerbyEvent (delegate Custom|QM%20Rotator) 0.01 true)
  (Audio|Components|Audio|Stop (Variables|Default|GetNetflix)))

(event Collision|EventActorBeginOverlap
  (params (OtherActor :type Actor%20Object%20Reference)))

(event EventTick
  (params (DeltaSeconds :type Float%20%28single-precision%29)))

(fn ConstructionScript)