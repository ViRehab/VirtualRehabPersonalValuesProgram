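; BP_Table is a demo-room actor that triggers a one-time hologram display on the UFO AI character when an actor overlaps it.
; After a short delay, it plays a grab sound and unhides the PSHologramBase02 component on the first AI_UFO_Character found in the level.
; A second delay keeps the hologram visible for several seconds before hiding it again.
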(event Collision|EventActorBeginOverlap
  (params (OtherActor :type Actor%20Object%20Reference))
  (Utilities|FlowControl|DoOnce false
    (:Completed
      (Utilities|FlowControl|Delay 1.0)
      (Audio|PlaySound2D "/Game/DemoRoom/Audio/Grab_Cue.Grab_Cue")
      (bind _outactors (Actor|GetAllActorsOfClass "/Game/DemoRoom/Character/AI_UFO_Character.AI_UFO_Character_C"))
      (Development|SetHiddeninGame (Variables|/Game/DemoRoom/Character/AI_UFO_Character.AI_UFO_Character_C|GetPS_HologramBase_02 (Utilities|Array|Get(acopy) _outactors)) false false)
      (Utilities|FlowControl|Delay 8.0)
      (bind _outactors_2 (Actor|GetAllActorsOfClass "/Game/DemoRoom/Character/AI_UFO_Character.AI_UFO_Character_C"))
      (Development|SetHiddeninGame (Variables|/Game/DemoRoom/Character/AI_UFO_Character.AI_UFO_Character_C|GetPS_HologramBase_02 (Utilities|Array|Get(acopy) _outactors_2)) true false))))

(fn ConstructionScript)